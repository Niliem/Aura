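; Anim notify that sends a gameplay event to the animated mesh's owner, named for triggering projectiles from animations.
; It sends the configured event tag with a projectile socket tag packed into the payload's InstigatorTags, so the receiver can read which socket is meant.
; The notify displays the event tag's name as its own name.
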(fn `GetNotifyName`
  (returns (ReturnValue :type String))
  (return (`KismetStringLibrary.Conv_NameToString` (`BlueprintGameplayTagLibrary.GetTagName` (`self.GameplayEventTag`)))))

(fn `Received_Notify`
  (params (MeshComp :type "SkeletalMeshComponent Object Reference") (Animation :type "AnimSequenceBase Object Reference") (EventReference :type "AnimNotifyEventReference Structure (by ref)"))
  (returns (ReturnValue :type Boolean))
  (`AbilitySystemBlueprintLibrary.SendGameplayEventToActor` (`ActorComponent.GetOwner` MeshComp) (`self.GameplayEventTag`) (make `GameplayEventData` (struct) null null null null (struct) (`BlueprintGameplayTagLibrary.MakeGameplayTagContainerFromTag` (`self.ProjectileSocket`))))
  (return true))