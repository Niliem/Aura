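; AN_HandleMelee is an anim notify that detects melee hits and reports them to the owning actor through a gameplay event.
; It gets the combat socket location for its socket tag, then gathers live AuraCharacterBase actors within the radius, ignoring the owner.
; Those actors are sent as target data under the configured event tag.
; The event tag also supplies the notify's display name.
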(fn `GetNotifyName`
  (returns (ReturnValue :type String))
  (return (`KismetStringLibrary.Conv_NameToString` (`BlueprintGameplayTagLibrary.GetTagName` (`self.GameplayEventTag`)))))

(fn `Received_Notify`
  (params (MeshComp :type "SkeletalMeshComponent Object Reference") (Animation :type "AnimSequenceBase Object Reference") (EventReference :type "AnimNotifyEventReference Structure (by ref)"))
  (returns (ReturnValue :type Boolean))
  (bind _returnvalue (`ActorComponent.GetOwner` MeshComp))
  (bind _returnvalue_2 (message `CombatInterface.GetCombatSocketLocation` _returnvalue (`self.SocketTag`)))
  (`AbilitySystemBlueprintLibrary.SendGameplayEventToActor` _returnvalue (`self.GameplayEventTag`) (make `GameplayEventData` (struct) null null null null (struct) (struct) (struct) 0.0 (`AbilitySystemBlueprintLibrary.AbilityTargetDataFromActorArray` (`AuraAbilitySystemLibrary.GetLiveActorsWithinRadius` _returnvalue "/Script/Aura.AuraCharacterBase" (`|MakeArray` _returnvalue) (`self.Radius`) _returnvalue_2))))
  (return true))