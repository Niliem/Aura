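; BP_EnemyBase is a base enemy character Blueprint that supplies the visual animation for spawning and dissolving.
; On BeginPlay a timeline drives a uniform scale on the mesh.
; Mesh and weapon dissolve events each run their own timeline into the Dissolve scalar parameter of the dynamic material instance passed in.
; SetFacingTarget feeds a location to Motion Warping as the FacingTarget warp target.
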(event `self.ReceiveBeginPlay`
  (bind (_direction _scale) (`Timeline|SpawnTimeline` :!via `PlayFromStart`)
    (:`Update`
      (`SceneComponent.SetRelativeScale3D` (`self.Mesh`) (`KismetMathLibrary.MakeVector` _scale _scale _scale)))))

(event `self.AnimateMeshDissolveMaterial`
  (params (DynamicMaterialInstance :type "MaterialInstanceDynamic Object Reference"))
  (bind (_direction _dissolvealpha) (`Timeline|MeshDissolveTimeline` :!via `PlayFromStart`)
    (:`Update`
      (`MaterialInstanceDynamic.SetScalarParameterValue` DynamicMaterialInstance "Dissolve" _dissolvealpha))))

(event `self.AnimateWeaponDissolveMaterial`
  (params (DynamicMaterialInstance :type "MaterialInstanceDynamic Object Reference"))
  (bind (_direction _dissolvealpha) (`Timeline|WeaponDissolveTimeline` :!via `PlayFromStart`)
    (:`Update`
      (`MaterialInstanceDynamic.SetScalarParameterValue` DynamicMaterialInstance "Dissolve" _dissolvealpha))))

(event `CombatInterface.SetFacingTarget`
  (params (TargetLocation :type "Vector Structure (by ref)"))
  (`MotionWarpingComponent.AddOrUpdateWarpTargetFromLocation` (`self.MotionWarping`) "FacingTarget" TargetLocation))

(fn `UserConstructionScript`)