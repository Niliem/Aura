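; Flame pillar actor that makes its fire light flicker.
; After a random start delay, a timeline plays an intensity curve, pausing briefly for a random time before each replay.
; A looping timer picks a random target offset, which Tick smooths toward with FInterpTo.
; Each timeline update combines the curve, base intensity and smoothed offset to set the light's intensity, varying the flicker.
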(event `self.ReceiveBeginPlay`
  (`KismetSystemLibrary.Delay` (`KismetMathLibrary.RandomFloatInRange` 0.2 1.0))
  (`KismetSystemLibrary.K2_SetTimerDelegate` (delegate `CustomEvent`) 1.2 true)
  (bind (_direction _flameintensity) (`Timeline|FlameIntensityTimeline` :!via `PlayFromStart` :!label _label)
    (:`Update`
      (`LightComponent.SetIntensity` (`self.FireLight`) (* (+ _flameintensity (/ (`self.CurrentOffset`) 2.0)) (`self.BaseIntensity`) (`self.CurrentOffset`))))
    (:`Finished`
      (`KismetSystemLibrary.Delay` (`KismetMathLibrary.RandomFloatInRange` 0.1 0.4))
      (goto _label :!via `PlayFromStart`))))

(event `CustomEvent`
  (set `self.TargetOffset` (`KismetMathLibrary.RandomFloatInRange` 0.8 1.2)))

(event `self.ReceiveTick`
  (params (DeltaSeconds :type "Float (single-precision)"))
  (set `self.CurrentOffset` (`KismetMathLibrary.FInterpTo` (`self.CurrentOffset`) (`self.TargetOffset`) DeltaSeconds 3.0)))

(fn `UserConstructionScript`)